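; BP_DirectPawn is a VR pawn for direct hand selection and grab-based world manipulation.
; BeginPlay adds the IMC_VR Enhanced Input mapping context to its player controller.
; Fore-pinch actions drive the left and right DirectSelector components, while grip, dolly and scale toggle actions forward to WorldGrabber.
; The construction script assigns each selector its hand sphere and gives WorldGrabber both hands, leaving interaction logic to those components.
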(event `self.ReceiveBeginPlay`
  ; Intialize Enhance Input
  (bind _asplayer_controller (cast `PlayerController` (`self.GetController`)))
  (message `EnhancedInputSubsystemInterface.AddMappingContext` (pcsubsystem `EnhancedInputLocalPlayerSubsystem` _asplayer_controller) "/Game/VAR_Class/Input/IMC_VR.IMC_VR" 0 (struct)))

(event `EnhancedInput|/Game/VAR_Class/Input/IA_LForePinch`
  (params (ActionValue :type Boolean) (ElapsedSeconds :type "Float (double-precision)") (TriggeredSeconds :type "Float (double-precision)") (InputAction :type "InputAction Object Reference" :default "/Game/VAR_Class/Input/IA_LForePinch.IA_LForePinch"))
  ; Intialize Left Fore Pitch
  (:`Triggered`
    (`Selector.ForePinch` (`self.LDirectSelector`) ActionValue)))

(event `EnhancedInput|/Game/VAR_Class/Input/IA_RForePinch`
  (params (ActionValue :type Boolean) (ElapsedSeconds :type "Float (double-precision)") (TriggeredSeconds :type "Float (double-precision)") (InputAction :type "InputAction Object Reference" :default "/Game/VAR_Class/Input/IA_RForePinch.IA_RForePinch"))
  ; Intialize Right Fore Pitch
  (:`Triggered`
    (`Selector.ForePinch` (`self.RDirectSelector`) ActionValue)))

(event `EnhancedInput|/Game/VAR_Class/Input/IA_LGrip`
  (params (ActionValue :type Boolean) (ElapsedSeconds :type "Float (double-precision)") (TriggeredSeconds :type "Float (double-precision)") (InputAction :type "InputAction Object Reference" :default "/Game/VAR_Class/Input/IA_LGrip.IA_LGrip"))
  ; Initalize World Grabber
  (:`Triggered`
    (`WorldGrabber.LWorldGrab` (`self.WorldGrabber`) ActionValue)))

(event `EnhancedInput|/Game/VAR_Class/Input/IA_RGrip`
  (params (ActionValue :type Boolean) (ElapsedSeconds :type "Float (double-precision)") (TriggeredSeconds :type "Float (double-precision)") (InputAction :type "InputAction Object Reference" :default "/Game/VAR_Class/Input/IA_RGrip.IA_RGrip"))
  ; Initalize World Grabber
  (:`Triggered`
    (`WorldGrabber.RWorldGrab` (`self.WorldGrabber`) ActionValue)))

(event `EnhancedInput|/Game/VAR_Class/Input/IA_DollyToggle`
  (params (ActionValue :type Boolean) (ElapsedSeconds :type "Float (double-precision)") (TriggeredSeconds :type "Float (double-precision)") (InputAction :type "InputAction Object Reference" :default "/Game/VAR_Class/Input/IA_DollyToggle.IA_DollyToggle"))
  ; Initalize World Grabber
  (:`Triggered`
    (`WorldGrabber.DollyToggle` (`self.WorldGrabber`) ActionValue)))

(event `EnhancedInput|/Game/VAR_Class/Input/IA_ScaleToggle`
  (params (ActionValue :type Boolean) (ElapsedSeconds :type "Float (double-precision)") (TriggeredSeconds :type "Float (double-precision)") (InputAction :type "InputAction Object Reference" :default "/Game/VAR_Class/Input/IA_ScaleToggle.IA_ScaleToggle"))
  ; Initalize World Grabber
  (:`Triggered`
    (`WorldGrabber.ScaleToggle` (`self.WorldGrabber`) ActionValue)))

(fn `UserConstructionScript`
  (bind _worldgrabber (`self.WorldGrabber`))
  ; Left Hand
  (set `Selector.hand` (`self.L Sphere`) (`self.LDirectSelector`))
  ; Right Hand
  (set `Selector.hand` (`self.R Sphere`) (`self.RDirectSelector`))
  (set `WorldGrabber.leftHand` (`self.L Hand`) _worldgrabber)
  (set `WorldGrabber.rightHand` (`self.R Hand`) _worldgrabber))